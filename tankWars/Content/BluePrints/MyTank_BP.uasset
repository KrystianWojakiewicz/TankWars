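; MyTank_BP is the player tank Blueprint, handling camera aiming and firing.
; On BeginPlay it passes its Barrel and TankTurret components to SetBarrel and SetTurret.
; Aim axes rotate the camera rig, with azimuth yawing AzimuthGimbal and elevation pitching SpringArm, so each axis turns a separate component.
; The Fire action calls Fire, which is defined outside these graphs.
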(event PhysicsVolumeChangedDelegate(Camera)
  (params (NewVolume :type Physics%20Volume%20Object%20Reference)))

(event EventBeginPlay
  (Class|Tank|SetBarrel (Variables|Default|GetBarrel))
  (Class|Tank|SetTurret (Variables|Default|GetTankTurret)))

(event Input|ActionEvents|InputActionFire
  (params (Key :type Key%20Structure))
  ;[1 1 1] Fire Projectile Input Binding
  (:Pressed
    (Class|Tank|Fire)))

(event Input|AxisEvents|InputAxisAimAzimuth
  (params (AxisValue :type Float%20%28single-precision%29))
  ;[1 1 1] Camera Input Binding
  (Transformation|AddLocalRotation (Variables|Default|GetAzimuthGimbal) (Math|Rotator|MakeRotator 0.0 0.0 AxisValue) false false))

(event Input|AxisEvents|InputAxisAimElevation
  (params (AxisValue :type Float%20%28single-precision%29))
  ;[1 1 1] Camera Input Binding
  (Transformation|AddLocalRotation (Variables|Default|GetSpringArm) (Math|Rotator|MakeRotator 0.0 AxisValue 0.0) false false))

(fn ConstructionScript)